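; Player-controlled Black Knight flipbook character for a side-view platformer, with Enhanced Input movement along X and jumping.
; Each tick, PlayerMoveAnimation picks idle, running, jumping or falling flipbooks from movement state, while control yaw flips with move direction.
; Roll launches along fixed world +X, but its animation branch is unreachable.
; A five-step light-attack combo is scaffolded but unwired from input; heavy and special attacks only print debug text.
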(event `self.ReceiveBeginPlay`
  (bind _asplayer_controller (cast `PlayerController` (`self.GetController`)))
  (`EnhancedInputSubsystemInterface.AddMappingContext` (pcsubsystem `EnhancedInputLocalPlayerSubsystem` _asplayer_controller) "/Game/Input/Player_Platform.Player_Platform" 0 (struct)))

(event `EnhancedInput|/Game/Input/Actions/Player_Jump`
  (params (ActionValue :type Boolean) (ElapsedSeconds :type "Float (double-precision)") (TriggeredSeconds :type "Float (double-precision)") (InputAction :type "InputAction Object Reference" :default "/Game/Input/Actions/Player_Jump.Player_Jump"))
  (:`Started`
    (`self.Jump`))
  (:`Completed`
    (`self.StopJumping`)))

(event `EnhancedInput|/Game/Input/Actions/Player_Move`
  (params (ActionValue :type "Float (double-precision)") (ElapsedSeconds :type "Float (double-precision)") (TriggeredSeconds :type "Float (double-precision)") (InputAction :type "InputAction Object Reference" :default "/Game/Input/Actions/Player_Move.Player_Move"))
  (:`Triggered`
    (`self.AddMovementInput` (1.0 0.0 0.0) ActionValue)
    (`Controller.SetControlRotation` (`self.GetController`) (select `bool` (> ActionValue 0.0) :`false` (`KismetMathLibrary.MakeRotator` 0.0 0.0 180.0) :`true` (`KismetMathLibrary.MakeRotator` 0.0)))))

(event `self.ReceiveTick`
  (params (DeltaSeconds :type "Float (single-precision)"))
  (`self.Player_Move_Animation`))

(event `EnhancedInput|/Game/Input/Actions/Player_Roll`
  (params (ActionValue :type Boolean) (ElapsedSeconds :type "Float (double-precision)") (TriggeredSeconds :type "Float (double-precision)") (InputAction :type "InputAction Object Reference" :default "/Game/Input/Actions/Player_Roll.Player_Roll"))
  (:`Started`
    (set `self.IsRolling` true)
    (`self.LaunchCharacter` (100.0 0.0 0.0) true)
    (`self.Player_Move_Animation`)
    (`KismetSystemLibrary.K2_SetTimerDelegate` :`Time` (`PaperFlipbookComponent.GetFlipbookLength` (`self.Sprite`)))))

(event `EnhancedInput|/Game/Input/Actions/Player_Atk_Heavy`
  (params (ActionValue :type Boolean) (ElapsedSeconds :type "Float (double-precision)") (TriggeredSeconds :type "Float (double-precision)") (InputAction :type "InputAction Object Reference" :default "/Game/Input/Actions/Player_Atk_Heavy.Player_Atk_Heavy"))
  (:`Triggered`
    (`KismetSystemLibrary.PrintString` "Heavy_Attack")))

(event `EnhancedInput|/Game/Input/Actions/Player_Atk_SP`
  (params (ActionValue :type Boolean) (ElapsedSeconds :type "Float (double-precision)") (TriggeredSeconds :type "Float (double-precision)") (InputAction :type "InputAction Object Reference" :default "/Game/Input/Actions/Player_Atk_SP.Player_Atk_SP"))
  (:`Triggered`
    (`KismetSystemLibrary.PrintString` "SP_Attack")))

(event `EnableQueue`
  (set `self.CanQueueNext` true))

(event `PlayerAtkL`
  (params (ComboIndex :type Boolean))
  (set `self.IsAttacking` true)
  (bind _output_get (set `self.CurrentComboIndex` (`KismetMathLibrary.Conv_BoolToInt` ComboIndex)))
  (switch `int` _output_get
    (:`1`
      (`PaperFlipbookComponent.SetFlipbook` (`self.Sprite`) "/Game/PaperAssets/Black_Knight/SpriteSheets_Separated/Attack_v1/BK_ATK_L1.BK_ATK_L1"))
    (:`2`
      (`PaperFlipbookComponent.SetFlipbook` (`self.Sprite`) "/Game/PaperAssets/Black_Knight/SpriteSheets_Separated/Attack_v1/BK_ATK_L2.BK_ATK_L2"))
    (:`3`
      (`PaperFlipbookComponent.SetFlipbook` (`self.Sprite`) "/Game/PaperAssets/Black_Knight/SpriteSheets_Separated/Attack_v1/BK_ATK_L3.BK_ATK_L3"))
    (:`4`
      (`PaperFlipbookComponent.SetFlipbook` (`self.Sprite`) "/Game/PaperAssets/Black_Knight/SpriteSheets_Separated/Attack_v1/BK_ATK_L4.BK_ATK_L4"))
    (:`5`
      (`PaperFlipbookComponent.SetFlipbook` (`self.Sprite`) "/Game/PaperAssets/Black_Knight/SpriteSheets_Separated/Attack_v1/BK_ATK_L5.BK_ATK_L5")))
  (`PaperFlipbookComponent.PlayFromStart` (`self.Sprite`)))

(event `ResetAtk`)

(event `EnhancedInput|/Game/Input/Actions/Player_Atk_Light`
  (params (ActionValue :type Boolean) (ElapsedSeconds :type "Float (double-precision)") (TriggeredSeconds :type "Float (double-precision)") (InputAction :type "InputAction Object Reference" :default "/Game/Input/Actions/Player_Atk_Light.Player_Atk_Light"))
  (:`Triggered`
    (if (`self.IsAttacking`)
      (if (`self.CanQueueNext`)
        _))))

(fn `Player_Move_Animation`
  (locals (NewLocalVar :type "PaperFlipbook Object Reference"))
  (bind (_returnvalue_x _returnvalue_y _returnvalue_z) (`KismetMathLibrary.BreakVector` (`self.GetVelocity`)))
  (if (`NavMovementComponent.IsMovingOnGround` (`self.CharacterMovement`))
    (if true
      (if (> (`KismetMathLibrary.VSize` (`self.GetVelocity`)) 0.0)
        (`PaperFlipbookComponent.SetFlipbook` (`self.Sprite`) "/Game/PaperAssets/Black_Knight/SpriteSheets_All/Caracter_with_FX/Black_Knight_Running.Black_Knight_Running")
        (else
          (`PaperFlipbookComponent.SetFlipbook` (`self.Sprite`) "/Game/PaperAssets/Black_Knight/SpriteSheets_Separated/Idle/Black_Knight_Idle_FB.Black_Knight_Idle_FB")))
      (elif (> (`KismetMathLibrary.VSize` (`self.GetVelocity`)) 0.0)
        (`PaperFlipbookComponent.SetFlipbook` (`self.Sprite`) "/Game/PaperAssets/Black_Knight/SpriteSheets_All/Caracter_with_FX/Black_Knight_Roll.Black_Knight_Roll")))
    (elif (< _returnvalue_z -100.0)
      (`PaperFlipbookComponent.SetFlipbook` (`self.Sprite`) "/Game/PaperAssets/Black_Knight/SpriteSheets_Separated/Fall_Light/Textures/Black_Knight_Fall.Black_Knight_Fall")
      (else
        (`PaperFlipbookComponent.SetFlipbook` (`self.Sprite`) "/Game/PaperAssets/Black_Knight/SpriteSheets_All/Caracter_with_FX/Black_Knight_Jumping.Black_Knight_Jumping")))))

(fn `UserConstructionScript`)