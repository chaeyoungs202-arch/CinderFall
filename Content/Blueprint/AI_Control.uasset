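; AI controller Blueprint shared by four enemy types (skeleton, goblin, shrooman and reyezer) that keeps its possessed pawn moving forward.
; On possess, it runs a cast for each type and stores the pawn in the matching typed variable.
; Each Tick, it calls MoveForward on whichever stored reference is valid, leaving the movement itself to the pawn classes.
; The reyezer cast lives in the generically named NewFunction.
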(event `self.ReceivePossess`
  (params (PossessedPawn :type "Pawn Object Reference"))
  (`self.Ai Skeleton` PossessedPawn)
  (`self.Ai Goblin` PossessedPawn)
  (`self.Ai shrooman` PossessedPawn)
  (`self.NewFunction` PossessedPawn))

(event `self.ReceiveTick`
  (params (DeltaSeconds :type "Float (single-precision)"))
  (`self.Ai Skeleton Forward`)
  (`self.Ai goblin forward`)
  (`self.Ai shrooman forward`)
  (`self.Ai reyezer forward`))

(fn `Ai Goblin`
  (params (Object :type "Object Object Reference"))
  (bind _asai_goblin (cast `/Game/Blueprint/AI_goblin` Object))
  (set `self.As AI Goblin` _asai_goblin))

(fn `Ai goblin forward`
  (bind _as_ai_goblin (`self.As AI Goblin`)
    (:`then`
      (`/Game/Blueprint/AI_goblin.MoveForward` _as_ai_goblin))
    (:`else`)))

(fn `Ai reyezer forward`
  (bind _as_ai_reyezer (`self.As AI Reyezer`)
    (:`then`
      (`/Game/Blueprint/AI_reyezer.MoveForward` _as_ai_reyezer))
    (:`else`)))

(fn `Ai shrooman`
  (params (Object :type "Object Object Reference"))
  (bind _asai_shrooman (cast `/Game/Blueprint/AI_shrooman` Object))
  (set `self.As AI Shrooman` _asai_shrooman))

(fn `Ai shrooman forward`
  (bind _as_ai_shrooman (`self.As AI Shrooman`)
    (:`then`
      (`/Game/Blueprint/AI_shrooman.MoveForward` _as_ai_shrooman))
    (:`else`)))

(fn `Ai Skeleton`
  (params (Object :type "Object Object Reference"))
  (bind _asai_skeleton (cast `/Game/Blueprint/AI_Skeleton` Object))
  (set `self.ControlledChar` _asai_skeleton))

(fn `Ai Skeleton Forward`
  (bind _controlledchar (`self.ControlledChar`)
    (:`then`
      (`/Game/Blueprint/AI_Skeleton.MoveForward` _controlledchar))
    (:`else`)))

(fn `NewFunction`
  (params (Object :type "Object Object Reference"))
  (bind _asai_reyezer (cast `/Game/Blueprint/AI_reyezer` Object))
  (set `self.As AI Reyezer` _asai_reyezer))

(fn `UserConstructionScript`)